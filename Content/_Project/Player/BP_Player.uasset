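; Player character Blueprint handling movement, camera look, running, interaction, inventory toggle and melee sword combat.
; On BeginPlay it hides weapon bones, spawns a holstered sword, creates the HUD and builds the inventory.
; The Sword input equips or unequips the sword; attach and equip events swap grip/holster sockets and switch between movement-oriented and controller-yaw rotation.
; State and combat-type enums are exposed through getter and setter functions.
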(event Input|ActionEvents|InputActionInventory
  (params (Key :type Key%20Structure))
  (bind _inventorycomponent (Variables|Default|GetInventoryComponent))
  (bind _widget (Variables|/Game/_Project/Components/InventoryComponent.InventoryComponent_C|GetWidget _inventorycomponent))
  (:Pressed
    (if (Widget|IsVisible _widget)
      (Widget|SetVisibility _widget "Hidden")
      (CallFunction|OffMouseCursor)
      (else
        (Widget|SetVisibility _widget "Visible")
        (CallFunction|OnMouseCursor)))))

(event Input|ActionEvents|InputActionInteraction
  (params (Key :type Key%20Structure))
  (:Pressed
    (Default|CallInteraction self)))

(fn ConstructionScript)

(fn OnMouseCursor
  (bind _returnvalue (Game|GetPlayerController 0))
  (Input|SetInputModeGameandUI _returnvalue (Variables|Default|GetHUD) "DoNotLock" true)
  (Variables|/Script/Engine.PlayerController|SetbShowMouseCursor _returnvalue true))

(fn OffMouseCursor
  (bind _returnvalue (Game|GetPlayerController 0))
  (Input|SetInputModeGameOnly _returnvalue)
  (Variables|/Script/Engine.PlayerController|SetbShowMouseCursor _returnvalue false))

(event EventBeginPlay
  (Utilities|FlowControl|Sequence
    (:then_0
      (|HideBone))
    (:then_1
      (|SpawnSword))
    (:then_2
      (bind _returnvalue (UserInterface|CreateWidget "/Game/_Project/Widgets/WB_HUD.WB_HUD_C" (Game|GetPlayerController 0)))
      (bind _output_get (Variables|Default|SetHUD _returnvalue))
      (UserInterface|Viewport|AddtoViewport _output_get 0)
      (Default|CreateInventory (Variables|Default|GetInventoryComponent)))))

(event Input|ActionEvents|InputActionRun
  (params (Key :type Key%20Structure))
  (bind _charactermovement (Variables|Character|GetCharacterMovement))
  ;[1 1 1] Run
  (:Pressed
    (Variables|/Script/Engine.CharacterMovementComponent|SetMaxWalkSpeed _charactermovement 6e+02))
  (:Released
    (Variables|/Script/Engine.CharacterMovementComponent|SetMaxWalkSpeed _charactermovement 2e+02)))

(event Input|AxisEvents|InputAxisMoveForward
  (params (AxisValue :type Float%20%28single-precision%29))
  ;[1 1 1] Movement
  (Pawn|Input|AddMovementInput (Math|Vector|GetForwardVector (Math|Rotator|MakeRotator 0.0 0.0 (.yaw (Pawn|GetControlRotation :!class /Script/Engine.Pawn)))) AxisValue false))

(event Input|AxisEvents|InputAxisMoveRight
  (params (AxisValue :type Float%20%28single-precision%29))
  ;[1 1 1] Movement
  (Pawn|Input|AddMovementInput (Math|Vector|GetRightVector (Math|Rotator|MakeRotator 0.0 0.0 (.yaw (Pawn|GetControlRotation :!class /Script/Engine.Pawn)))) AxisValue false))

(event Input|AxisEvents|InputAxisHorizontalLook
  (params (AxisValue :type Float%20%28single-precision%29))
  ;[1 1 1] Camera Mouse Rotation
  (Pawn|Input|AddControllerYawInput AxisValue))

(event Input|AxisEvents|InputAxisVerticalLook
  (params (AxisValue :type Float%20%28single-precision%29))
  ;[1 1 1] Camera Mouse Rotation
  (Pawn|Input|AddControllerPitchInput AxisValue))

(event Input|ActionEvents|InputActionAttack
  (params (Key :type Key%20Structure))
  (:Pressed
    (bind _currentweapon (Variables|Default|GetCurrentWeapon)
      (:then
        (Default|Attack _currentweapon))
      (:else))))

(event Custom|Equipped
  ;[1 1 1] Equip Melee Weapon
  (Variables|Default|SetStateType "NewEnumerator0")
  (Variables|Default|SetCombatType "NewEnumerator1")
  (Variables|Default|SetbUseControllerRotationYaw true)
  (Variables|/Script/Engine.CharacterMovementComponent|SetbOrientRotationToMovement (Variables|Character|GetCharacterMovement) false))

(event Custom|Unequipped
  ;[1 1 1] Unequip Melee Weapon
  (Variables|Default|SetStateType "NewEnumerator0")
  (Variables|Default|SetCombatType "NewEnumerator0")
  (Variables|Default|SetbUseControllerRotationYaw false)
  (Variables|/Script/Engine.CharacterMovementComponent|SetbOrientRotationToMovement (Variables|Character|GetCharacterMovement) true))

(event Custom|AttachMeleeWeapon
  (Transformation|AttachComponentToComponent (Variables|Default|GetSword) (Variables|Character|GetMesh) "Weapon_Melee_OneHand_Grip" "KeepRelative" "KeepRelative" "KeepRelative" true))

(event Custom|DettachMeleeWeapon
  (Transformation|AttachComponentToComponent (Variables|Default|GetSword) (Variables|Character|GetMesh) "Weapon_Melee_OneHand_Holster" "KeepRelative" "KeepRelative" "KeepRelative" true))

(event Input|ActionEvents|InputActionSword
  (params (Key :type Key%20Structure))
  (:Pressed
    (bind _currentweapon (Variables|Default|GetCurrentWeapon)
      (:then
        (if (== _currentweapon (Variables|Default|GetSword))
          (Default|Unequip (Variables|Default|GetCurrentWeapon))
          (Variables|Default|SetCurrentWeapon 0)
          (else
            (bind _output_get (Variables|Default|SetCurrentWeapon (Variables|Default|GetSword)))
            (Default|Equip _output_get))))
      (:else
        (bind _output_get_2 (Variables|Default|SetCurrentWeapon (Variables|Default|GetSword)))
        (Default|Equip _output_get_2)))))

(fn GetCombatType
  (return (Variables|Default|GetCombatType)))

(fn GetCurrentWeapon
  (return (Variables|Default|GetCurrentWeapon)))

(fn Hitted
  (Variables|Default|SetStateType "NewEnumerator8")
  (return false))

(fn IsStateAttacking
  (return (Utilities|Enum|Equal(Enum) (Variables|Default|GetStateType) "NewEnumerator3")))

(fn IsStateIdling
  (return (Utilities|Enum|Equal(Enum) (Variables|Default|GetStateType) "NewEnumerator0")))

(fn SetCanMove
  (params (InCanMove :type Boolean))
  (Variables|Default|SetCanMove InCanMove)
  (return false))

(fn SetCurrentWeapon
  (params (NewWeapon :type BP%20Weapon%20Object%20Reference))
  (Utilities|IsValid (Variables|Default|GetCurrentWeapon)
    (:Is%20Valid
      (Default|OnUnequipped (Variables|Default|GetCurrentWeapon)))
    (:Is%20Not%20Valid
      _))
  (Utilities|IsValid NewWeapon
    (:Is%20Valid
      (bind _output_get (Variables|Default|SetCurrentWeapon NewWeapon))
      (Default|OnEquipped _output_get)
      (return _output_get))
    (:Is%20Not%20Valid
      (Variables|Default|SetCurrentWeapon 0)
      (return 0))))

(fn SetStateAttacking
  (Variables|Default|SetStateType "NewEnumerator3")
  (return false))

(fn SetStateIdling
  (Variables|Default|SetStateType "NewEnumerator0")
  (return false))

(fn SetStateSpelling
  (Variables|Default|SetStateType "NewEnumerator7")
  (return false))

(fn WeaponAttach
  (CallFunction|AttachMeleeWeapon)
  (return false))

(fn WeaponDettach
  (CallFunction|DettachMeleeWeapon)
  (return false))

(fn WeaponEquipped
  (CallFunction|Equipped)
  (return false))

(fn WeaponUnequipped
  (CallFunction|Unequipped)
  (return false))