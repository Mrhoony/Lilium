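; Player actor for the main menu that puts the first player controller into UI-only input and displays the menu widget.
; BeginPlay sets the input mode without mouse lock.
; While OnMainMenu is true, Tick creates WB_MainMenu if the stored reference is invalid, then adds it to the viewport.
; Nodes that hide or show the menu are present but unconnected, so they never run.
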(event EventBeginPlay
  (Input|SetInputModeUIOnly (Game|GetPlayerController 0) 0 "DoNotLock"))

(event Collision|EventActorBeginOverlap
  (params (OtherActor :type Actor%20Object%20Reference)))

(event EventTick
  (params (DeltaSeconds :type Float%20%28single-precision%29))
  (if (Variables|Default|GetOnMainMenu)
    (bind _mainmenu (Variables|Default|GetMainMenu)
      (:then)
      (:else
        (bind _returnvalue (UserInterface|CreateWidget "/Game/_Project/Widgets/WB_MainMenu.WB_MainMenu_C" (Game|GetPlayerController 0)))
        (bind _output_get (Variables|Default|SetMainMenu _returnvalue))
        (UserInterface|Viewport|AddtoViewport _output_get 0)))))

(fn ConstructionScript)