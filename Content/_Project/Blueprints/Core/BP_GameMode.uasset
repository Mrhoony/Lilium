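; Game mode that ends a mission by showing a fail screen when the player dies or a complete screen when the boss dies.
; BeginPlay caches the BP_Player and BP_Boss actors found in the level.
; Tick polls each one's StatusComponent for death and adds the matching widget to the viewport.
; A shared IsFinishGame flag allows only one result, with player death checked first.
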(event EventBeginPlay
  (bind _returnvalue (Actor|GetActorOfClass "/Game/_Project/Player/BP_Player.BP_Player_C"))
  (Variables|Default|SetPlayer _returnvalue)
  (bind _returnvalue_2 (Actor|GetActorOfClass "/Game/_Project/Boss/BP_Boss.BP_Boss_C"))
  (Variables|Default|SetBoss _returnvalue_2))

(event EventTick
  (params (DeltaSeconds :type Float%20%28single-precision%29))
  (bind _returnvalue (Game|GetPlayerController 0))
  (bind _boss (Variables|Default|GetBoss))
  (bind _player (Variables|Default|GetPlayer))
  (Utilities|FlowControl|Sequence
    (:then_0
      (Utilities|IsValid _player
        (:Is%20Valid
          (if (and (Math|Boolean|Equal(Boolean) (Variables|Default|GetIsFinishGame) false) (Default|IsDead (Variables|/Game/_Project/Player/BP_Player.BP_Player_C|GetStatusComponent _player)))
            (bind _returnvalue_2 (UserInterface|CreateWidget "/Game/_Project/Widgets/WB_MissionFail.WB_MissionFail_C" _returnvalue))
            (UserInterface|Viewport|AddtoViewport _returnvalue_2 0)
            (Variables|Default|SetIsFinishGame true :!label _label)))))
    (:then_1
      (Utilities|IsValid _boss
        (:Is%20Valid
          (if (and (Math|Boolean|Equal(Boolean) (Variables|Default|GetIsFinishGame) false) (Default|IsDead (Variables|/Game/_Project/Boss/BP_Boss.BP_Boss_C|GetStatusComponent _boss)))
            (bind _returnvalue_3 (UserInterface|CreateWidget "/Game/_Project/Widgets/WB_MissionComplete.WB_MissionComplete_C" _returnvalue))
            (UserInterface|Viewport|AddtoViewport _returnvalue_3 0)
            (goto _label)))))))

(fn ConstructionScript)