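; BP_Posion_Test is a pickup item actor, apparently a test potion, that the player can collect into their inventory.
; Entering its Sphere binds a PickUp event to the BP_Player's interaction, and leaving the sphere unbinds it.
; PickUp adds the item's Icon and its own class to the player's InventoryComponent, refreshes the inventory, then destroys the actor.
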(event OnComponentBeginOverlap(Sphere)
  (params (OverlappedComponent :type Primitive%20Component%20Object%20Reference) (OtherActor :type Actor%20Object%20Reference) (OtherComp :type Primitive%20Component%20Object%20Reference) (OtherBodyIndex :type Integer) (bFromSweep :type Boolean) (SweepResult :type Hit%20Result%20Structure%20%28by%20ref%29))
  (bind _asbp_player (Utilities|Casting|CastToBP_Player OtherActor))
  (EventDispatchers|BindEventtoInteraction _asbp_player (delegate Custom|PickUp)))

(event OnComponentEndOverlap(Sphere)
  (params (OverlappedComponent :type Primitive%20Component%20Object%20Reference) (OtherActor :type Actor%20Object%20Reference) (OtherComp :type Primitive%20Component%20Object%20Reference) (OtherBodyIndex :type Integer))
  (bind _asbp_player (Utilities|Casting|CastToBP_Player OtherActor))
  (EventDispatchers|UnbindEventfromInteraction _asbp_player (delegate Custom|PickUp)))

(event Custom|PickUp
  (params (OtherActor :type Actor%20Object%20Reference))
  (bind _asbp_player (Utilities|Casting|CastToBP_Player OtherActor))
  (Default|AddItemtoInventory (Variables|/Game/_Project/Player/BP_Player.BP_Player_C|GetInventoryComponent _asbp_player) (Variables|Default|GetIcon) (Utilities|GetClass self))
  (Default|RefreshInventory (Variables|/Game/_Project/Player/BP_Player.BP_Player_C|GetInventoryComponent _asbp_player))
  (Actor|DestroyActor))

(event EventBeginPlay)

(event Collision|EventActorBeginOverlap
  (params (OtherActor :type Actor%20Object%20Reference)))

(event EventTick
  (params (DeltaSeconds :type Float%20%28single-precision%29)))

(fn ConstructionScript)