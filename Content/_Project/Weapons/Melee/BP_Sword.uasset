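; BP_Sword is a melee weapon Blueprint that damages actors overlapping its capsule hitbox, using its Power value.
; The capsule's collision starts disabled and is switched on and off through the OnCollision and OffCollision events.
; Equip and Unequip set the owning BP_Player's state type and play the matching montage on it.
; Each event calls its parent implementation first, extending a base weapon class.
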(event OnComponentBeginOverlap(Capsule)
  (params (OverlappedComponent :type Primitive%20Component%20Object%20Reference) (OtherActor :type Actor%20Object%20Reference) (OtherComp :type Primitive%20Component%20Object%20Reference) (OtherBodyIndex :type Integer) (bFromSweep :type Boolean) (SweepResult :type Hit%20Result%20Structure%20%28by%20ref%29))
  ;[1 1 1] Overlap
  (CallFunction|SendDamage OtherActor (Variables|Default|GetPower)))

(event EventBeginPlay
  ;[1 1 1] BeginPlay
  (|CallParentFunction)
  (Collision|SetCollisionEnabled (Variables|Default|GetCapsule) "NoCollision"))

(event EventOnCollision
  ;[1 1 1] Collision
  (|CallParentFunction)
  (Collision|SetCollisionEnabled (Variables|Default|GetCapsule) "QueryAndPhysics"))

(event EventOffCollision
  ;[1 1 1] Collision
  (|CallParentFunction)
  (Collision|SetCollisionEnabled (Variables|Default|GetCapsule) "NoCollision"))

(event EventEquip
  ;[1 1 1] Equip
  (|CallParentFunction)
  (bind _asbp_player (Utilities|Casting|CastToBP_Player (Components|GetOwner)))
  (Variables|/Game/_Project/Player/BP_Player.BP_Player_C|SetStateType _asbp_player "NewEnumerator1")
  (Animation|PlayAnimMontage _asbp_player "/Game/_Project/Player/Montages/Sword/Sword_Equip_Montage.Sword_Equip_Montage" 1.0 "None"))

(event EventUnequip
  ;[1 1 1] Unequip
  (|CallParentFunction)
  (bind _asbp_player (Utilities|Casting|CastToBP_Player (Components|GetOwner)))
  (Variables|/Game/_Project/Player/BP_Player.BP_Player_C|SetStateType _asbp_player "NewEnumerator2")
  (Animation|PlayAnimMontage _asbp_player "/Game/_Project/Player/Montages/Sword/Sword_Unequip_Montage.Sword_Unequip_Montage" 1.0 "None"))

(fn ConstructionScript
  (|CallParentFunction))