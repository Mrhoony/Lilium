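; AI controller for the boss that starts its behavior tree and keeps track of the player through AI perception.
; On possess, it casts the pawn to BP_Boss and runs the BehaviorTree assigned on that pawn, if valid.
; Each perception update scans currently perceived actors for a BP_Player, writing the first found to the PlayerKey blackboard key, or clearing the key when none is found.
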(event OnPerceptionUpdated(AIPerception)
  (params (UpdatedActors :type Array%20of%20Actor%20Object%20References))
  (|Find&RegisterPlayerinBlackBoard))

(event EventBeginPlay)

(event EventTick
  (params (DeltaSeconds :type Float%20%28single-precision%29)))

(event EventPossess
  (params (PossessedPawn :type Pawn%20Object%20Reference))
  (bind _asbp_boss (Utilities|Casting|CastToBP_Boss PossessedPawn))
  (bind _output_get (Variables|Default|SetAIPawn _asbp_boss))
  (bind _behaviortree (Variables|/Game/_Project/Boss/BP_Boss.BP_Boss_C|GetBehaviorTree _output_get)
    (:then
      (AI|RunBehaviorTree _behaviortree))
    (:else)))

(fn ConstructionScript)

(event Custom|PerceptionBreak
  (Utilities|Array|ForEachLoopwithBreak (Class|AIPerceptionComponent|GetCurrentlyPerceivedActors (Variables|Default|GetAIPerception))) ; enters at Break
)