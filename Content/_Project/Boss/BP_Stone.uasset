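; BP_Stone is a stone projectile from the Boss folder that is launched toward a target location.
; On BeginPlay it disables collision on its static mesh, and nothing in the graph turns it back on.
; Fire sets the projectile movement velocity toward the target at Speed, applies reduced gravity, activates the component and gives the actor a short lifespan.
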(event Custom|Fire
  (params (TargetLocation :type Vector))
  (bind _projectilemovement (Variables|Default|GetProjectileMovement))
  (Variables|/Script/Engine.MovementComponent|SetVelocity _projectilemovement (* (Math|Vector|Normalize (- TargetLocation (Transformation|GetActorLocation))) (Variables|Default|GetSpeed)))
  (Variables|/Script/Engine.ProjectileMovementComponent|SetProjectileGravityScale _projectilemovement 0.2)
  (Components|Activation|Activate _projectilemovement false)
  (Actor|SetLifeSpan 3.0))

(event EventBeginPlay
  (Collision|SetCollisionEnabled (Variables|Default|GetStaticMesh) "NoCollision"))

(fn ConstructionScript)