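; Boss character with three cooldown-gated attacks: random data-table melee montages, a thrown stone, and a charge at the player.
; Tick counts down cooldowns, turns the stationary boss toward the player using a cross-product sign, and drives the charge until its collision overlaps.
; Damage lowers StatusComponent health and flashes dynamic materials; death ragdolls the mesh away from the attacker, then destroys the actor.
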(fn ConstructionScript
  (|SetDynamicMaterials))

(fn SetBodyColor
  (params (InLinearColor :type Linear%20Color%20Structure))
  (for _array_element (Variables|Default|GetDynamicMaterials)
    (Rendering|Material|SetVectorParameterValue _array_element "BaseColor" InLinearColor :!class /Script/Engine.MaterialInstanceDynamic)))

(fn Ragdoll
  (bind _mesh (Variables|Character|GetMesh))
  (Collision|SetCollisionEnabled (Variables|Collision|GetCapsuleComponent) "NoCollision")
  (Variables|/Script/Engine.SkeletalMeshComponent|SetGlobalAnimRateScale _mesh 0.0)
  (Physics|SetSimulatePhysics _mesh true)
  (Collision|SetCollisionEnabled _mesh "QueryAndPhysics")
  (Physics|AddForce _mesh (* (* (Math|Vector|GetUnitDirection(Vector) (Transformation|GetActorLocation (Variables|Default|GetAttacker)) (Transformation|GetActorLocation)) (Variables|Default|GetDamage)) 1e+05) "None" false))

(fn Turn
  (Variables|Default|SetStateType "NewEnumerator12")
  (return))

(fn EndAttack
  (Variables|Default|SetStateType "NewEnumerator0")
  (bind _asbp_boss_controller (Utilities|Casting|CastToBP_BossController (Pawn|GetController)))
  (AI|ClearFocus _asbp_boss_controller)
  (Variables|Default|SetCrash false))

(fn AttackMelee
  (bind _returnvalue (Math|Random|RandomIntegerinRange 0 2))
  (bind _meleedatas (Variables|Default|GetMeleeDatas))
  (bind _output (Utilities|Array|Get(acopy) _meleedatas _returnvalue))
  (if (== (Variables|CoolTimes|GetCT_curMelee) 0.0)
    (Variables|Default|SetStateType "NewEnumerator3")
    (Animation|PlayAnimMontage (.montage _output) (.playrate _output) (.startsection _output))
    (Variables|CoolTimes|SetCT_curMelee (Variables|CoolTimes|GetCT_maxMelee))
    (return (.montage _output))))

(fn AttackThrow
  (Variables|Default|SetStateType "NewEnumerator3")
  (Animation|PlayAnimMontage "/Game/_Project/Boss/Montages/Attack_Throw_Ready_Montage.Attack_Throw_Ready_Montage" 1.0 "None")
  (Variables|CoolTimes|SetCT_curThrow (Variables|CoolTimes|GetCT_maxThrow))
  (return))

(fn AttackThrowReady
  (bind _returnvalue (Game|SpawnActorfromClass "/Game/_Project/Boss/BP_Stone.BP_Stone_C" (Math|Transform|MakeTransform "0, 0, 0") "Undefined" 0 0))
  (bind _output_get (Variables|Default|SetStone _returnvalue))
  (Utilities|IsValid _output_get
    (:Is%20Valid
      (Transformation|AttachComponentToComponent _output_get (Variables|Character|GetMesh) "Throw_Stone" "KeepRelative" "KeepRelative" "SnapToTarget" true)
      (return false))
    (:Is%20Not%20Valid
      (return false))))

(fn AttackThrowFire
  (Utilities|IsValid (Variables|Default|GetStone)
    (:Is%20Valid
      (Variables|Default|SetTargetLocation (Transformation|GetActorLocation (Game|GetPlayerCharacter 0)))
      (bind _asbp_boss_controller (Utilities|Casting|CastToBP_BossController (Pawn|GetController)))
      (AI|SetFocus _asbp_boss_controller (Game|GetPlayerCharacter 0))
      (Transformation|DetachFromActor (Variables|Default|GetStone) "KeepWorld" "KeepWorld" "KeepWorld")
      (Default|Fire (Variables|Default|GetStone) (Variables|Default|GetTargetLocation)))))

(fn AttackCrash
  (Variables|Default|SetStateType "NewEnumerator3")
  (Animation|PlayAnimMontage "/Game/_Project/Boss/Montages/Attack_Crash_Ready_Montage.Attack_Crash_Ready_Montage" 1.0 "None")
  (Variables|CoolTimes|SetCT_curCrash (Variables|CoolTimes|GetCT_maxCrash))
  (return))

(fn AttackCrashFire
  (Variables|Default|SetStateType "NewEnumerator3")
  (Variables|Default|SetCrash true)
  (Variables|Default|SetTargetLocation (Math|Vector|GetUnitDirection(Vector) (Transformation|GetActorLocation) (Transformation|GetActorLocation (Game|GetPlayerCharacter 0))))
  (Animation|PlayAnimMontage "/Game/_Project/Boss/Montages/Attack_Crash_Fire_Montage.Attack_Crash_Fire_Montage" 1.0 "None"))

(event OnComponentBeginOverlap(CrashCollision)
  (params (OverlappedComponent :type Primitive%20Component%20Object%20Reference) (OtherActor :type Actor%20Object%20Reference) (OtherComp :type Primitive%20Component%20Object%20Reference) (OtherBodyIndex :type Integer) (bFromSweep :type Boolean) (SweepResult :type Hit%20Result%20Structure%20%28by%20ref%29))
  (if (Variables|Default|GetCrash)
    (CallFunction|EndAttack)))

(event Game|Damage|EventAnyDamage
  (params (Damage :type Float%20%28single-precision%29) (DamageType :type Damage%20Type%20Object%20Reference) (InstigatedBy :type Controller%20Object%20Reference) (DamageCauser :type Actor%20Object%20Reference))
  (|SetDamage InstigatedBy Damage DamageCauser)
  (Class|NavMovementComponent|StopMovementKeepPathing (Variables|Character|GetCharacterMovement))
  (Animation|PlayAnimMontage 0 1.0 "None")
  (|HitColor)
  (|CheckDead) ; 삭제예정 : `보스 HP가 0이하일 시 죽는 시네마틱 실행`으로 변경
)

(event EventTick
  (params (DeltaSeconds :type Float%20%28single-precision%29))
  (Utilities|FlowControl|Sequence
    (:then_0
      (|UpdateCoolTimes))
    (:then_1
      (|GetCrossProduct))
    (:then_2
      (|ExecuteTurn))
    (:then_3
      (|ExecuteCrash))))

(event EventBeginPlay
  (Utilities|FlowControl|Sequence
    (:then_0
      (|GetOriginalMaterialBaseColor))
    (:then_1
      (|GetMeleeAttack))))

(fn Hitted
  (return false))

(fn IsStateAttacking
  (return false))

(fn IsStateIdling
  (return (Utilities|Enum|Equal(Enum) (Variables|Default|GetStateType) "NewEnumerator0")))

(fn SetCanMove
  (params (InCanMove :type Boolean))
  (return false))

(fn SetStateAttacking
  (return false))

(fn SetStateIdling
  (return false))

(fn SetStateSpelling
  (return false))